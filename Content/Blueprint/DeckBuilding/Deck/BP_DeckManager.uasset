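; Deck manager Blueprint for a deck-building game, currently a debug-level prototype of card drawing.
; PiocherCarte (draw card) runs on BeginPlay and on each G key press.
; It prints the name of the Deck entry at TopDeckIndex and advances the index without removing the card, or prints a not-found message once the index is invalid.
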(event `Key|G`
  (params (Key :type "Key Structure"))
  (:`Pressed`
    (`self.Piocher Carte` :!label _label)))

(event `self.ReceiveBeginPlay`
  (goto _label))

(fn `Piocher Carte`
  (bind _deck (`self.Deck`))
  (bind _topdeckindex (`self.TopDeckIndex`))
  (bind _output_nom (break `/Game/Blueprint/DeckBuilding/Struct/S_CarteData` (`|GetArrayItem` _deck _topdeckindex)))
  (if (`KismetArrayLibrary.Array_IsValidIndex` _deck _topdeckindex)
    (`KismetSystemLibrary.PrintString` _output_nom)
    (`/Engine/EditorBlueprintResources/StandardMacros.IncrementInt` (`self.TopDeckIndex`))
    (else
      (`KismetSystemLibrary.PrintString` "CartePasTrouvé"))))

(fn `UserConstructionScript`)