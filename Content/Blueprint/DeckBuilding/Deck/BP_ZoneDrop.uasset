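; BP_ZoneDrop is a drop zone in the deck-building card game that validates the card placed in it.
; Overlap events use BPI_Cartes to track the card inside and set or clear that card's current zone.
; ValidéLaCarte looks up the card's name in Liste; on a match, it repeatedly calls SuppTouteLesCartes on BP_GIDeck, then triggers dialogue through BP_GMDeck.
; Query functions identify it as a drop zone, not a card.
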(event `self.ReceiveBeginPlay`
  (bind _asbp_gideck (cast `/Game/Blueprint/Core/BP_GIDeck` (`GameplayStatics.GetGameInstance`)))
  (set `self.As BP GIDeck` _asbp_gideck)
  (bind _asbp_gmdeck (cast `/Game/Blueprint/Core/BP_GMDeck` (`GameplayStatics.GetGameMode`)))
  (set `self.As BP GMDeck` _asbp_gmdeck))

(event `self.ZoneDrop.OnComponentBeginOverlap`
  (params (OverlappedComponent :type "PrimitiveComponent Object Reference") (OtherActor :type "Actor Object Reference") (OtherComp :type "PrimitiveComponent Object Reference") (OtherBodyIndex :type Integer) (bFromSweep :type Boolean) (SweepResult :type "HitResult Structure (by ref)"))
  (bind (_estunecarte _carte) (message `/Game/Blueprint/BPI/BPI_Cartes.EstUneCarte` OtherActor))
  (if (`KismetSystemLibrary.DoesImplementInterface` OtherActor "/Game/Blueprint/BPI/BPI_Cartes.BPI_Cartes_C")
    (set `self.CarteDansZone` _carte)
    (set `/Game/Blueprint/DeckBuilding/Deck/BP_Cartes.ZoneActuel` self _carte)))

(event `self.ZoneDrop.OnComponentEndOverlap`
  (params (OverlappedComponent :type "PrimitiveComponent Object Reference") (OtherActor :type "Actor Object Reference") (OtherComp :type "PrimitiveComponent Object Reference") (OtherBodyIndex :type Integer))
  (bind (_estunecarte _carte) (message `/Game/Blueprint/BPI/BPI_Cartes.EstUneCarte` OtherActor))
  (if (`KismetSystemLibrary.DoesImplementInterface` OtherActor "/Game/Blueprint/BPI/BPI_Cartes.BPI_Cartes_C")
    (set `self.CarteDansZone` null)
    (set `/Game/Blueprint/DeckBuilding/Deck/BP_Cartes.ZoneActuel` null _carte)))

(fn `EstUneCarte`
  (returns (EstUneCarte :type Boolean) (carte :type "/Game/Blueprint/DeckBuilding/Deck/BP_Cartes Object Reference"))
  (return false null))

(fn `UserConstructionScript`)

(fn `ValidéLaCarte`
  (bind _cartedanszone (`self.CarteDansZone`))
  (bind _liste (`self.Liste`))
  (bind _cartedata_nom (break `/Game/Blueprint/DeckBuilding/Struct/S_CarteData` (`/Game/Blueprint/DeckBuilding/Deck/BP_Cartes.CarteData` _cartedanszone)))
  (bind _keys (`BlueprintMapLibrary.Map_Keys` _liste))
  (if (`.ReturnValue` (`BlueprintMapLibrary.Map_Find` _liste _cartedata_nom))
    (`/Game/Blueprint/Core/BP_GIDeck.SuppTouteLesCartes` (`self.As BP GIDeck`) _cartedanszone)
    (`/Game/Blueprint/Core/BP_GIDeck.SuppTouteLesCartes` (`self.As BP GIDeck`) null)
    (`/Game/Blueprint/Core/BP_GIDeck.SuppTouteLesCartes` (`self.As BP GIDeck`) null)
    (`/Game/Blueprint/Core/BP_GIDeck.SuppTouteLesCartes` (`self.As BP GIDeck`) null)
    (`/Game/Blueprint/Core/BP_GIDeck.SuppTouteLesCartes` (`self.As BP GIDeck`) null)
    (`/Game/Blueprint/Core/BP_GIDeck.SuppTouteLesCartes` (`self.As BP GIDeck`) null)
    (`/Game/Blueprint/Core/BP_GMDeck.CallDialogue` (`self.As BP GMDeck`))))

(fn `ZoneDeDrop`
  (returns (ZoneDeDrop :type "/Game/Blueprint/DeckBuilding/Deck/BP_ZoneDrop Object Reference") (EstUneZoneDeDrop :type Boolean))
  (return self true))