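; Card actor for the deck-building game that can be hovered, zoomed and dragged into a zone.
; On BeginPlay it slides to a hand offset and rotation from BP_GIDeck, then stores that base pose.
; Hover lifts and outlines it and registers it with the GameInstance, unless a flag locks it during moves, zoom or drag.
; Tick drags it along a clamped cursor trace; release validates ZoneActuel or snaps back.
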(event `MouvDéZoom`
  (bind (_baseplace_x _baseplace_y _baseplace_z) (`KismetMathLibrary.BreakVector` (`self.BasePlace`)))
  (`KismetSystemLibrary.MoveComponentTo` (`self.DefaultSceneRoot`) (`KismetMathLibrary.MakeVector` _baseplace_x _baseplace_y _baseplace_z) (`KismetMathLibrary.MakeRotator` -10.0 (`self.BaseY`) 90.0))
  (set `self.JeT'overlapPlusSalePute` false)
  (`SceneComponent.SetVisibility` (`self.PlaneContour`) false false))

(event `MouvZoom`
  (bind (_placevisu_x _placevisu_y _placevisu_z) (`KismetMathLibrary.BreakVector` (`self.PlaceVisu`)))
  (set `self.JeT'overlapPlusSalePute` true)
  (`KismetSystemLibrary.MoveComponentTo` (`self.DefaultSceneRoot`) (`KismetMathLibrary.MakeVector` _placevisu_x _placevisu_y _placevisu_z) (`KismetMathLibrary.MakeRotator` -10.0 0.0 90.0))
  (`SceneComponent.SetVisibility` (`self.PlaneContour`) false false))

(event `self.Box.OnEndCursorOver`
  (params (TouchedComponent :type "PrimitiveComponent Object Reference"))
  (bind _returnvalue (`self.GetTransform`))
  (bind (_baseplace_x _baseplace_y _baseplace_z) (`KismetMathLibrary.BreakVector` (`self.BasePlace`)))
  (bind _as_bp_gideck (`self.As BP GIDeck`))
  (if (not (`self.JeT'overlapPlusSalePute`))
    (set `/Game/Blueprint/Core/BP_GIDeck.canVisu` false _as_bp_gideck)
    (set `/Game/Blueprint/Core/BP_GIDeck.CarteOverlapp` null _as_bp_gideck)
    (`SceneComponent.SetVisibility` (`self.PlaneContour`) false false)
    (`KismetSystemLibrary.MoveComponentTo` (`self.DefaultSceneRoot`) (`KismetMathLibrary.MakeVector` (.x (.location _returnvalue)) (.y (.location _returnvalue)) _baseplace_z) (`KismetMathLibrary.MakeRotator` (.roll (.rotation _returnvalue)) (.pitch (.rotation _returnvalue)) (.yaw (.rotation _returnvalue))) false false 0.25)))

(event `self.ReceiveBeginPlay`
  (bind _returnvalue (`self.GetTransform`))
  (bind _asbp_gideck (cast `/Game/Blueprint/Core/BP_GIDeck` (`GameplayStatics.GetGameInstance`)))
  (bind _output_get (set `self.As BP GIDeck` _asbp_gideck))
  (set `self.JeT'overlapPlusSalePute` true)
  (bind (_x _y _z) (`/Game/Blueprint/Core/BP_GIDeck.CalculOffSet` _output_get))
  (bind _y_2 (`/Game/Blueprint/Core/BP_GIDeck.CalculRota` _output_get))
  (`KismetSystemLibrary.MoveComponentTo` (`self.DefaultSceneRoot`) (`KismetMathLibrary.MakeVector` _x _y _z) (`KismetMathLibrary.MakeRotator` (.roll (.rotation _returnvalue)) _y_2 (.yaw (.rotation _returnvalue))) false false 1.25)
  (`KismetSystemLibrary.Delay` 1.3)
  (set `self.BasePlace` (.location _returnvalue))
  (set `self.BaseY` (.pitch (.rotation _returnvalue)))
  (set `self.JeT'overlapPlusSalePute` false))

(event `self.Box.OnBeginCursorOver`
  (params (TouchedComponent :type "PrimitiveComponent Object Reference"))
  (bind _returnvalue (`self.GetTransform`))
  (bind (_baseplace_x _baseplace_y _baseplace_z) (`KismetMathLibrary.BreakVector` (`self.BasePlace`)))
  (if (not (`self.JeT'overlapPlusSalePute`))
    (set `/Game/Blueprint/Core/BP_GIDeck.canVisu` true (`self.As BP GIDeck`))
    (set `/Game/Blueprint/Core/BP_GIDeck.CarteOverlapp` self (`self.As BP GIDeck`))
    (`SceneComponent.SetVisibility` (`self.PlaneContour`) true false)
    (`KismetSystemLibrary.MoveComponentTo` (`self.DefaultSceneRoot`) (`KismetMathLibrary.MakeVector` (.x (.location _returnvalue)) (.y (.location _returnvalue)) (+ _baseplace_z 1.25)) (`KismetMathLibrary.MakeRotator` (.roll (.rotation _returnvalue)) (.pitch (.rotation _returnvalue)) (.yaw (.rotation _returnvalue))) false false 0.25)))

(event `self.Box.OnReleased`
  (params (TouchedComponent :type "PrimitiveComponent Object Reference") (ButtonReleased :type "Key Structure"))
  (bind _planecontour (`self.PlaneContour`))
  (bind _zoneactuel (`self.ZoneActuel`))
  (bind _output_get (set `self.EstEnDrag` false))
  (`ActorComponent.SetComponentTickEnabled` (`self.Box`) _output_get)
  ;[0.15 0.001747 0 0.5] A définir
  (if (!= _zoneactuel null)
    (`self.K2_SetActorLocation` (`self.K2_GetActorLocation` _zoneactuel))
    (`SceneComponent.SetVisibility` _planecontour false false)
    (`/Game/Blueprint/DeckBuilding/Deck/BP_ZoneDrop.ValidéLaCarte` (`self.ZoneActuel`))
    (else
      (set `self.JeT'overlapPlusSalePute` false)
      (`self.K2_SetActorTransform` (`KismetMathLibrary.MakeTransform` (`self.BasePlace`) (`KismetMathLibrary.MakeRotator` -10.0 (`self.BaseY`) 90.0) (0.25 0.25 0.25)))
      (`SceneComponent.SetVisibility` _planecontour false false))))

(event `self.Box.OnClicked`
  (params (TouchedComponent :type "PrimitiveComponent Object Reference") (ButtonPressed :type "Key Structure"))
  (set `self.JeT'overlapPlusSalePute` true)
  (`KismetSystemLibrary.PrintString` "j'ai cliqué")
  (bind _output_get (set `self.EstEnDrag` true))
  (`ActorComponent.SetComponentTickEnabled` (`self.Box`) _output_get))

(event `self.ReceiveTick`
  (params (DeltaSeconds :type "Float (single-precision)"))
  (bind _returnvalue_x (`KismetMathLibrary.BreakVector` (`self.K2_GetActorLocation`)))
  (bind _hitresult (`PlayerController.GetHitResultUnderCursorByChannel` (`GameplayStatics.GetPlayerController` 0) "TraceTypeQuery1" true))
  (if (`self.EstEnDrag`)
    (`self.K2_SetActorTransform` (`KismetMathLibrary.MakeTransform` (`KismetMathLibrary.MakeVector` _returnvalue_x (`KismetMathLibrary.FClamp` (.y (`.Location` (`GameplayStatics.BreakHitResult` _hitresult))) -20.0 20.0) (`KismetMathLibrary.FClamp` (.z (`.Location` (`GameplayStatics.BreakHitResult` _hitresult))) 590.0 620.0)) (struct :`Yaw` 90.0 :`Roll` -10.0) (0.25 0.25 0.25)))))

(fn `EstUneCarte`
  (returns (EstUneCarte :type Boolean) (carte :type "/Game/Blueprint/DeckBuilding/Deck/BP_Cartes Object Reference"))
  (return true self))

(fn `UserConstructionScript`)