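; Player controller for the card deck mode, handling input for card zoom, drawing and dialogue skipping.
; Zoom toggles the overlapped card held in BP_GIDeck, zooming in only while viewing is allowed.
; A one-shot, gated first draw calls BP_GMDeck, while PiocherLesCartes draws through the game instance with drag-and-drop mouse input disabled until a delay ends.
; Dialogue skip advances the game mode's dialogue widget when more pages remain.
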(event `InputAction|ZoomCarte`
  (params (Key :type "Key Structure"))
  (bind _inzoom (`self.InZoom`))
  (bind _as_bp_gideck (`self.As BP GIDeck`))
  (bind _carteoverlapp (`/Game/Blueprint/Core/BP_GIDeck.CarteOverlapp` _as_bp_gideck))
  (:`Pressed`
    (if (`/Game/Blueprint/Core/BP_GIDeck.canVisu` _as_bp_gideck)
      (if _inzoom
        (`/Game/Blueprint/DeckBuilding/Deck/BP_Cartes.MouvDéZoom` _carteoverlapp)
        (set `self.InZoom` false)
        (else
          (`/Game/Blueprint/DeckBuilding/Deck/BP_Cartes.MouvZoom` _carteoverlapp)
          (set `self.InZoom` true)))
      (elif _inzoom
        (`/Game/Blueprint/DeckBuilding/Deck/BP_Cartes.MouvDéZoom` _carteoverlapp)
        (set `self.InZoom` false)))))

(event `T'asIntere`
  (if (`self.Autorized`) :!label _label
    (`/Engine/EditorBlueprintResources/StandardMacros.DoOnce` false
      (:`Completed`
        (`/Game/Blueprint/Core/BP_GMDeck.1erPechPhase1` (`self.As BP GMDeck`))
        (`KismetSystemLibrary.Delay` 1.6)
        (`self.ACtiveD&D`)))))

(event `InputAction|PiocherUneCarte`
  (params (Key :type "Key Structure"))
  (:`Pressed`
    (goto _label)))

(event `self.ReceiveBeginPlay`
  (bind _asbp_gideck (cast `/Game/Blueprint/Core/BP_GIDeck` (`GameplayStatics.GetGameInstance`)))
  (set `self.As BP GIDeck` _asbp_gideck)
  (`self.ACtiveD&D`)
  (bind _asbp_gmdeck (cast `/Game/Blueprint/Core/BP_GMDeck` (`GameplayStatics.GetGameMode`)))
  (set `self.As BP GMDeck` _asbp_gmdeck))

(event `PiocherLesCartes`
  (`self.DesactiveD&D`)
  (`/Game/Blueprint/Core/BP_GIDeck.PiocherCarte` (`self.As BP GIDeck`))
  (`KismetSystemLibrary.Delay` 1.6)
  (`self.ACtiveD&D`))

(event `ACtiveD&D`
  (set `self.bShowMouseCursor` true)
  (set `self.bEnableMouseOverEvents` true)
  (set `self.bEnableClickEvents` true))

(event `DesactiveD&D`
  (set `self.bShowMouseCursor` false)
  (set `self.bEnableMouseOverEvents` false)
  (set `self.bEnableClickEvents` false))

(event `InputAction|Skip dialogue`
  (params (Key :type "Key Structure"))
  (bind _wbdia (`/Game/Blueprint/Core/BP_GMDeck.WBDIa` (`self.As BP GMDeck`)))
  (:`Pressed`
    (if (`/Game/Blueprint/Widgets/WB_DialogueText.MoreDIalogue?` _wbdia)
      (`/Game/Blueprint/Widgets/WB_DialogueText.PassPage` _wbdia))))

(fn `UserConstructionScript`)