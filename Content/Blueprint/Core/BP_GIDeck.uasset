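; BP_GIDeck manages the card deck: building it, drawing cards, clearing them and creating the HUD on the Tuto event.
; InitialiserLeDeck fills Deck from DataTableCartes rows; PiocherCarte spawns the next entry as a typed BP_Cartes and tracks it.
; Helpers derive camera-relative offset and pitch from hand count, with ScrennCam using the offset to spawn BP_TapisScreen.
; SuppTouteLesCartes destroys the given card, clears the list and conditionally removes one BPI_CarteID actor.
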(event `Tuto`
  (bind _asbp_gmdeck (cast `/Game/Blueprint/Core/BP_GMDeck` (`GameplayStatics.GetGameMode`)))
  (set `self.As BP GMDeck` _asbp_gmdeck)
  (bind _returnvalue (`|CreateWidget` "/Game/Blueprint/Widgets/WB_HUD.WB_HUD_C"))
  (bind _output_get (set `self.Hud` _returnvalue))
  (`UserWidget.AddToViewport` _output_get 0))

(fn `CalculOffSet`
  (returns (x :type "Float (double-precision)") (y :type "Float (double-precision)") (z :type "Float (double-precision)"))
  (bind _cartesrestantemain (`self.CartesRestanteMain`))
  (bind (_ecartcam_x _ecartcam_y _ecartcam_z) (`KismetMathLibrary.BreakVector` (`self.EcartCam`)))
  (bind (_returnvalue_x _returnvalue_y _returnvalue_z) (`KismetMathLibrary.BreakVector` (`Actor.K2_GetActorLocation` (`GameplayStatics.GetPlayerCameraManager` 0))))
  (bind _returnvalue (* _cartesrestantemain 0.5))
  (if (>= _cartesrestantemain 3)
    (set `self.ZTrans` (+ _ecartcam_z (+ (- _returnvalue_z _returnvalue) 2.0)))
    (else
      (set `self.ZTrans` (+ (+ _returnvalue _returnvalue_z) _ecartcam_z))))
  (return (+ (+ (* (`self.CartesRestanteMain`) 0.5) _returnvalue_x) _ecartcam_x) (+ (- _returnvalue_y (* _cartesrestantemain 2.5)) _ecartcam_y) (`self.ZTrans`)))

(fn `CalculRota`
  (returns (y :type "Float (double-precision)"))
  (bind (_returnvalue_roll _returnvalue_pitch) (`KismetMathLibrary.BreakRotator` (`Actor.K2_GetActorRotation` (`GameplayStatics.GetPlayerCameraManager` 0))))
  (bind _output_get (set `self.YRota` (+ (- _returnvalue_pitch 15.0) (* (`self.CartesRestanteMain`) 10))))
  (return _output_get))

(fn `InitialiserLeDeck`
  (bind _datatablecartes (`self.DataTableCartes`))
  (`KismetSystemLibrary.PrintString` "Je M'init")
  (`KismetArrayLibrary.Array_Clear` (`self.Deck`))
  (set `self.CartesRestanteDeck` 0)
  (bind _outrownames (`DataTableFunctionLibrary.GetDataTableRowNames` _datatablecartes))
  (bind _output_get (set `self.ActualRowNamesCartes` _outrownames))
  (for _array_element _output_get
    (bind _returnvalue (`|GetDataTableRow` _datatablecartes _array_element)
      (:`then`
        (`KismetArrayLibrary.Array_Add` (`self.Deck`) _returnvalue)
        (`KismetSystemLibrary.PrintString` "Loop de la liste"))
      (:`RowNotFound`
        (`KismetSystemLibrary.PrintString` "PasTrouvé De Row" true true (struct :`R` 1.0 :`G` 0.049562 :`A` 1.0)))))
  (set `self.TopDeckIndex` 0)
  (set `self.CartesRestanteDeck` (`KismetArrayLibrary.Array_Length` (`self.Deck`))))

(fn `PiocherCarte`
  (returns (carte :type "/Game/Blueprint/DeckBuilding/Deck/BP_Cartes Object Reference"))
  (bind _topdeckindex (`self.TopDeckIndex`))
  (if (> (`KismetArrayLibrary.Array_Length` (`self.Deck`)) _topdeckindex)
    (`KismetSystemLibrary.PrintString` "Je Pioche")
    (bind _returnvalue (`|SpawnActorFromClass` "/Game/Blueprint/DeckBuilding/Deck/BP_Cartes.BP_Cartes_C" (`KismetMathLibrary.MakeTransform` (-4550.0 650.0 480.0) (struct :`Yaw` 90.0 :`Roll` -10.0) (0.25 0.25 0.25)) "AdjustIfPossibleButAlwaysSpawn" "MultiplyWithRoot" null (`|GetArrayItem` (`self.Deck`) _topdeckindex) null))
    (set `/Game/Blueprint/DeckBuilding/Deck/BP_Cartes.E_Type` (`BlueprintMapLibrary.Map_Find` (`self.ListeDesNom`) (`self.AllCardCount`)) _returnvalue)
    (`/Engine/EditorBlueprintResources/StandardMacros.IncrementInt` (`self.AllCardCount`)
      (:`  `
        (`KismetArrayLibrary.Array_Add` (`self.ListeCarteSpawn`) _returnvalue)
        (`/Engine/EditorBlueprintResources/StandardMacros.IncrementInt` (`self.TopDeckIndex`)
          (:`  `
            (`/Engine/EditorBlueprintResources/StandardMacros.IncrementInt` (`self.CartesRestanteMain`)
              (:`  `
                (return _returnvalue)))))))
    (else
      (`KismetSystemLibrary.PrintString` "Je Pioche Pas" true true (struct :`R` 1.0 :`G` 0.021217 :`A` 1.0)))))

(fn `scrennCam`
  (bind (_x _y _z) (`self.CalculOffSet`))
  (`|SpawnActorFromClass` "/Game/Blueprint/Interaction/BP_TapisScreen.BP_TapisScreen_C" (`KismetMathLibrary.MakeTransform` (`KismetMathLibrary.MakeVector` (- _x 4600.0) _y _z) (struct :`Yaw` 90.0)) "AlwaysSpawn" "MultiplyWithRoot" null null))

(fn `SuppTouteLesCartes`
  (params (carte :type "/Game/Blueprint/DeckBuilding/Deck/BP_Cartes Object Reference"))
  (bind _carddestroy (`self.cardDestroy`))
  (`Actor.K2_DestroyActor` carte)
  (`KismetArrayLibrary.Array_Clear` (`self.ListeCarteSpawn`))
  (bind _outactors (`GameplayStatics.GetAllActorsWithInterface` "/Game/Blueprint/BPI/BPI_CarteID.BPI_CarteID_C"))
  (if (not (== (`KismetArrayLibrary.Array_Length` _outactors) _carddestroy))
    (`Actor.K2_DestroyActor` (`.ReturnValue` (`GameplayStatics.FindNearestActor` (0.0 0.0 0.0) _outactors)))
    (`/Engine/EditorBlueprintResources/StandardMacros.IncrementInt` _carddestroy
      (:`  `
        (set `self.CartesRestanteMain` 0)))))